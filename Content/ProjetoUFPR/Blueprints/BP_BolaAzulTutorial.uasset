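; BP_BolaAzulTutorial is a tutorial blue ball actor that is destroyed when the left and right pincers (BP_Pinca_E, BP_Pinca_D) both touch it in quick succession.
; Sphere overlaps compare against the first actor of each pincer class and raise crossed flags (E sets PincaD, D sets PincaE).
; Each flag clears after its own, unequal delay; the ball is destroyed when both are true.
; A Timeline for wobbling movement is never triggered.
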(event `self.ReceiveBeginPlay`
  (bind (_returnvalue_x _returnvalue_y) (`KismetMathLibrary.BreakVector` (`SceneComponent.K2_GetComponentLocation` (`self.DefaultSceneRoot`))))
  (set `self.PincaD` false)
  (set `self.PincaE` false)
  (set `self.Return Value Y` _returnvalue_y)
  (set `self.Return Value X` _returnvalue_x))

(event `self.Sphere.OnComponentBeginOverlap`
  (params (OverlappedComponent :type "PrimitiveComponent Object Reference") (OtherActor :type "Actor Object Reference") (OtherComp :type "PrimitiveComponent Object Reference") (OtherBodyIndex :type Integer) (bFromSweep :type Boolean) (SweepResult :type "HitResult Structure (by ref)"))
  (bind _outactors (`GameplayStatics.GetAllActorsOfClass` "/Game/ProjetoUFPR/Blueprints/BP_Pinca_E.BP_Pinca_E_C"))
  (if (== (`|GetArrayItem` _outactors) OtherActor)
    (`self.D_true`)
    (`self.Both_True`)
    (else
      (bind _outactors_2 (`GameplayStatics.GetAllActorsOfClass` "/Game/ProjetoUFPR/Blueprints/BP_Pinca_D.BP_Pinca_D_C"))
      (if (== OtherActor (`|GetArrayItem` _outactors_2))
        (`self.E_true`)
        (`self.Both_True`)))))

(event `D_true`
  (set `self.PincaD` true)
  (`KismetSystemLibrary.Delay` 5.0)
  (set `self.PincaD` false))

(event `E_true`
  (set `self.PincaE` true)
  (`KismetSystemLibrary.Delay` 0.5)
  (set `self.PincaE` false))

(event `Both_True`
  (if (== (`self.PincaE`) (`self.PincaD`))
    (if (== true (`self.PincaD`))
      (`self.K2_DestroyActor`))))

(fn `UserConstructionScript`)