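; BP_BolaAzul is a blue ball that rides a track and is destroyed when caught by two pincers.
; On BeginPlay, one timeline moves it along the BP_BallsTrack spline from a randomised playback position, while another adds vertical offset.
; Sphere overlaps with either pincer set temporary flags, and the ball destroys itself when both are true.
; Score and remaining-ball events exist but are not called in the live destroy path.
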(event `self.ReceiveBeginPlay`
  (bind _returnvalue (`GameplayStatics.GetActorOfClass` "/Game/ProjetoUFPR/Blueprints/BP_BallsTrack.BP_BallsTrack_C"))
  (set `self.TrackRef` _returnvalue)
  (`self.Move Ball`)
  (set `self.PincaD` false)
  (set `self.PincaE` false))

(event `Move Ball`
  (bind (_returnvalue_x _returnvalue_y _returnvalue_z) (`KismetMathLibrary.BreakVector` (`SplineComponent.GetLocationAtDistanceAlongSpline` (`/Game/ProjetoUFPR/Blueprints/BP_BallsTrack.Spline` (`self.TrackRef`)) (`KismetMathLibrary.Lerp` 0.0 (`SplineComponent.GetSplineLength` (`/Game/ProjetoUFPR/Blueprints/BP_BallsTrack.Spline` (`self.TrackRef`))) (`self.Alfa`)) "World")))
  ;[1 0 0] Evento para deixar a blinha na spline
  (`|ExecutionSequence`
    (:`then_0`
      (`TimelineComponent.SetPlaybackPosition` (`self.Ball Mover`) (`KismetMathLibrary.RandomFloatInRange` 0.0 (`SplineComponent.GetSplineLength` (`/Game/ProjetoUFPR/Blueprints/BP_BallsTrack.Spline` (`self.TrackRef`)))) false true)
      (`TimelineComponent.SetPlayRate` (`self.Ball Mover`) (/ 1.0 (`self.Duration Ball Mover`)))
      (bind (_direction _alfa) (`Timeline|Ball Mover`)
        (:`Update`
          (set `self.Alfa` _alfa)
          (`self.K2_SetActorTransform` (`KismetMathLibrary.MakeTransform` (`KismetMathLibrary.MakeVector` _returnvalue_x _returnvalue_y _returnvalue_z))))))
    (:`then_1`
      ;;[1 1 1] Playrate do Eixo Z
      (`TimelineComponent.SetPlayRate` (`self.Timeline EixoZ`) (/ 1.0 (`self.DurationEixoZ`)))
      (bind (_direction_2 _eixo_z) (`Timeline|Timeline EixoZ`)
        (:`Update`
          (bind _output_get (set `self.Eixo Z` _eixo_z))
          (`self.K2_AddActorWorldOffset` (`KismetMathLibrary.MakeVector` 0.0 0.0 _output_get)))))))

(event `BolasAzuis`
  (bind _outactors (`GameplayStatics.GetAllActorsOfClass` "BP_BolaAzul_C"))
  (bind _returnvalue (== (`KismetArrayLibrary.Array_Length` _outactors) 0))
  (if _returnvalue
    (set `self.TemAzul` _returnvalue)))

(event `AddPontosBlue`
  (bind _asbp_game_mode_main (`/Game/AFCore/Libraries/FLib_Core.getMainGameMode` (`GameplayStatics.GetGameMode`)))
  (`/Game/AFCore/Blueprints/Game/BP_GameMode_Main.Pontoslevel` _asbp_game_mode_main))

(event `self.Sphere.OnComponentBeginOverlap`
  (params (OverlappedComponent :type "PrimitiveComponent Object Reference") (OtherActor :type "Actor Object Reference") (OtherComp :type "PrimitiveComponent Object Reference") (OtherBodyIndex :type Integer) (bFromSweep :type Boolean) (SweepResult :type "HitResult Structure (by ref)"))
  (if (== (`self.Ref_PincaE`) OtherActor)
    (`self.D_true`)
    (`self.Both_True`)
    (elif (== OtherActor (`self.Ref_PincaD`))
      (`self.E_true`)
      (`self.Both_True`))))

(event `D_true`
  (set `self.PincaD` true)
  (`KismetSystemLibrary.Delay` 5.0)
  (set `self.PincaD` false))

(event `E_true`
  (set `self.PincaE` true)
  (`KismetSystemLibrary.Delay` 0.5)
  (set `self.PincaE` false))

(event `Both_True`
  (if (== (`self.PincaE`) (`self.PincaD`))
    (if (== true (`self.PincaD`))
      (`self.K2_DestroyActor`))))

(fn `UserConstructionScript`)