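; BP_Pinca_D is a pincer part, likely the right one, that detects contact with the blue ball (Bolaazul).
; Box begin and end overlaps set and clear the EncostouD flag for that ball, printing each change on screen.
; A looping timer started at BeginPlay runs ChecarVelocidade, which prints the Box's physics angular speed whenever it exceeds a threshold.
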(event `self.ReceiveBeginPlay`
  (`parent.ReceiveBeginPlay`)
  (`KismetSystemLibrary.K2_SetTimer` null "ChecarVelocidade" 0.1 true))

(event `self.ReceiveTick`
  (params (DeltaSeconds :type "Float (single-precision)")))

(event `self.Box.OnComponentBeginOverlap`
  (params (OverlappedComponent :type "PrimitiveComponent Object Reference") (OtherActor :type "Actor Object Reference") (OtherComp :type "PrimitiveComponent Object Reference") (OtherBodyIndex :type Integer) (bFromSweep :type Boolean) (SweepResult :type "HitResult Structure (by ref)"))
  (if (== OtherActor (`self.Bolaazul`))
    (bind _output_get (set `self.EncostouD` true))
    (`KismetSystemLibrary.PrintString` (`KismetStringLibrary.Conv_BoolToString` _output_get) true true (struct :`G` 1.0 :`B` 0.01975 :`A` 1.0) 0.2)))

(event `self.Box.OnComponentEndOverlap`
  (params (OverlappedComponent :type "PrimitiveComponent Object Reference") (OtherActor :type "Actor Object Reference") (OtherComp :type "PrimitiveComponent Object Reference") (OtherBodyIndex :type Integer))
  (if (== OtherActor (`self.Bolaazul`))
    (bind _output_get (set `self.EncostouD` false))
    (`KismetSystemLibrary.PrintString` (`KismetStringLibrary.Conv_BoolToString` _output_get) true true (struct :`G` 1.0 :`B` 0.01975 :`A` 1.0) 0.2)))

(fn `ChecarVelocidade`
  (bind _returnvalue (`KismetMathLibrary.VSize` (`PrimitiveComponent.GetPhysicsAngularVelocityInDegrees` (`self.Box`) "None")))
  (if (> _returnvalue 50.0)
    (`KismetSystemLibrary.PrintString` (`KismetStringLibrary.Conv_DoubleToString` _returnvalue))))

(fn `UserConstructionScript`
  (`parent.UserConstructionScript`))