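; BP_Config holds the score and level progression for a ball-based training game.
; Pontuacao adjusts Pontos by counting ball actors in the world, subtracting blue, green and red balls and adding death balls.
; IniciarTreinamento switches to the first stage data asset through the main game instance.
; MudarLevel switches to SettedLevel, then increments IndexLevel to preselect the following level from DALevelList.
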(event `Pontuacao`
  ;[1 1 1] SISTEMA DE PONTOS
  (bind _outactors (`GameplayStatics.GetAllActorsOfClass` "/Game/ProjetoUFPR/Blueprints/BP_BolaAzul.BP_BolaAzul_C"))
  (set `self.Pontos` (- (`self.Pontos`) (`KismetArrayLibrary.Array_Length` _outactors)))
  (bind _outactors_2 (`GameplayStatics.GetAllActorsOfClass` "/Game/ProjetoUFPR/Blueprints/BP_BolaVerde.BP_BolaVerde_C"))
  (set `self.Pontos` (- (`self.Pontos`) (`KismetArrayLibrary.Array_Length` _outactors_2)))
  (bind _outactors_3 (`GameplayStatics.GetAllActorsOfClass` "/Game/ProjetoUFPR/Blueprints/BP_BolaVermelha.BP_BolaVermelha_C"))
  (set `self.Pontos` (- (`self.Pontos`) (`KismetArrayLibrary.Array_Length` _outactors_3)))
  (bind _outactors_4 (`GameplayStatics.GetAllActorsOfClass` "/Game/ProjetoUFPR/Blueprints/BP_BolaMorte.BP_BolaMorte_C"))
  (set `self.Pontos` (+ (`self.Pontos`) (`KismetArrayLibrary.Array_Length` _outactors_4))))

(event `self.ReceiveBeginPlay`)

(event `Iniciar Treinamento`
  (bind _gameinstance (`/Game/AFCore/Libraries/FLib_Core.getMainGameInstance` (`GameplayStatics.GetGameInstance`)))
  (`/Game/AFCore/Blueprints/Game/BP_GameInstance_Main.SwitchLevel` _gameinstance "/Game/ProjetoUFPR/DataAssets/Level/Nivel_1/DA_N1Etapa1.DA_N1Etapa1" false false))

(event `Mudar Level`
  (bind _gameinstance (`/Game/AFCore/Libraries/FLib_Core.getMainGameInstance` (`GameplayStatics.GetGameInstance`)))
  (`/Game/AFCore/Blueprints/Game/BP_GameInstance_Main.SwitchLevel` _gameinstance (`self.Setted_Level`) false false)
  (bind _result (`/Engine/EditorBlueprintResources/StandardMacros.IncrementInt` (`self.Index_Level`))
    (:`  `
      (set `self.Setted_Level` (`|GetArrayItem` (`self.DA_Level_List`) _result)))))

(fn `UserConstructionScript`)