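; BP_Pinca_Start1 is a grabbable tweezers (pinça) actor that destroys itself at BeginPlay if the game instance's Pegou flag is already set.
; Its Box overlap events set EncostouD while touching Bolaazul and print the value for debugging.
; Comp_Grab pickup and activation only print "Hello".
; The logic that would set Pegou, destroy the actor and switch to DA_nivel1 is disconnected and never runs.
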(event `self.ReceiveBeginPlay`
  (`parent.ReceiveBeginPlay`)
  (bind _gameinstance (`/Game/AFCore/Libraries/FLib_Core.getMainGameInstance` (`GameplayStatics.GetGameInstance`)))
  (if (`/Game/AFCore/Blueprints/Game/BP_GameInstance_Main.Pegou` _gameinstance)
    (`self.K2_DestroyActor`)))

(event `self.Box.OnComponentBeginOverlap`
  (params (OverlappedComponent :type "PrimitiveComponent Object Reference") (OtherActor :type "Actor Object Reference") (OtherComp :type "PrimitiveComponent Object Reference") (OtherBodyIndex :type Integer) (bFromSweep :type Boolean) (SweepResult :type "HitResult Structure (by ref)"))
  (if (== OtherActor (`self.Bolaazul`))
    (bind _output_get (set `self.EncostouD` true))
    (`KismetSystemLibrary.PrintString` (`KismetStringLibrary.Conv_BoolToString` _output_get) true true (struct :`G` 1.0 :`B` 0.01975 :`A` 1.0) 0.2)))

(event `self.Box.OnComponentEndOverlap`
  (params (OverlappedComponent :type "PrimitiveComponent Object Reference") (OtherActor :type "Actor Object Reference") (OtherComp :type "PrimitiveComponent Object Reference") (OtherBodyIndex :type Integer))
  (if (== OtherActor (`self.Bolaazul`))
    (bind _output_get (set `self.EncostouD` false))
    (`KismetSystemLibrary.PrintString` (`KismetStringLibrary.Conv_BoolToString` _output_get) true true (struct :`G` 1.0 :`B` 0.01975 :`A` 1.0) 0.2)))

(event `self.Comp_Grab.Grab_ActorPickedUp`
  (params (GrabbingPawn :type "/Game/AFCore/Blueprints/Pawn/BP_Pawn_Base Object Reference") (GrabbingActor :type "Actor Object Reference"))
  (`KismetSystemLibrary.PrintString` "Hello" :!label _label))

(event `self.Comp_Grab.OnComponentActivated`
  (params (Component :type "ActorComponent Object Reference") (bReset :type Boolean))
  (goto _label))

(event `self.Comp_Grab.Grab_Thumbstick`
  (params (UpAxis :type "Float (single-precision)") (RightAxis :type "Float (single-precision)")))

(event `self.Comp_Grab.Grab_ActorReleased`
  (params (ReleasingPawn :type "/Game/AFCore/Blueprints/Pawn/BP_Pawn_Base Object Reference") (ReleasingActor :type "Actor Object Reference") (LastRelease :type Boolean)))

(event `self.Comp_Grab.Grab_TriggerAxis`
  (params (TriggerAxis :type "Float (single-precision)")))

(event `self.Comp_Grab.OnComponentDeactivated`
  (params (Component :type "ActorComponent Object Reference")))

(event `self.Comp_Grab.Grab_Highlight`
  (params (ImpactLocation :type "Vector Structure") (ImpactRotation :type "Rotator Structure") (ImpactComponent :type "ActorComponent Object Reference") (Pawn :type "/Game/AFCore/Blueprints/Pawn/BP_Pawn_Base Object Reference") (MotionComponent :type "/Game/AFCore/Blueprints/VR/MotionComponents/BP_MComp Object Reference")))

(event `self.Comp_Grab.Grab_GripAxis`
  (params (GripAxis :type "Float (single-precision)")))

(event `self.Comp_Grab.Grab_KeyInput`
  (params (Key :type "/Game/AFCore/Enums/Enum_Controller_Buttons Enum" :default "NewEnumerator1") (Set :type Boolean)))

(fn `UserConstructionScript`
  (`parent.UserConstructionScript`))