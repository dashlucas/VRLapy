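; BP_Pinca_Start is a grabbable start pickup (a "pinça", or tweezers) that launches the first level when picked up.
; The grab event sets the Pegou flag on the main game instance, destroys the actor and switches to DA_nivel1 with fade and server travel.
; On BeginPlay the actor destroys itself if that flag is already set.
; A box overlap with Bolaazul toggles EncostouD and prints it, without affecting the pickup.
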(event `self.ReceiveBeginPlay`
  (`parent.ReceiveBeginPlay`)
  (bind _gameinstance (`/Game/AFCore/Libraries/FLib_Core.getMainGameInstance` (`GameplayStatics.GetGameInstance`)))
  (if (`/Game/AFCore/Blueprints/Game/BP_GameInstance_Main.Pegou` _gameinstance)
    (`self.K2_DestroyActor`)))

(event `self.Box.OnComponentBeginOverlap`
  (params (OverlappedComponent :type "PrimitiveComponent Object Reference") (OtherActor :type "Actor Object Reference") (OtherComp :type "PrimitiveComponent Object Reference") (OtherBodyIndex :type Integer) (bFromSweep :type Boolean) (SweepResult :type "HitResult Structure (by ref)"))
  (if (== OtherActor (`self.Bolaazul`))
    (bind _output_get (set `self.EncostouD` true))
    (`KismetSystemLibrary.PrintString` (`KismetStringLibrary.Conv_BoolToString` _output_get) true true (struct :`G` 1.0 :`B` 0.01975 :`A` 1.0) 0.2)))

(event `self.Box.OnComponentEndOverlap`
  (params (OverlappedComponent :type "PrimitiveComponent Object Reference") (OtherActor :type "Actor Object Reference") (OtherComp :type "PrimitiveComponent Object Reference") (OtherBodyIndex :type Integer))
  (if (== OtherActor (`self.Bolaazul`))
    (bind _output_get (set `self.EncostouD` false))
    (`KismetSystemLibrary.PrintString` (`KismetStringLibrary.Conv_BoolToString` _output_get) true true (struct :`G` 1.0 :`B` 0.01975 :`A` 1.0) 0.2)))

(event `self.Comp_Grab.Grab_ActorPickedUp`
  (params (GrabbingPawn :type "/Game/AFCore/Blueprints/Pawn/BP_Pawn_Base Object Reference") (GrabbingActor :type "Actor Object Reference"))
  (`KismetSystemLibrary.PrintString` "Pegou")
  (bind _gameinstance (`/Game/AFCore/Libraries/FLib_Core.getMainGameInstance` (`GameplayStatics.GetGameInstance`)))
  (set `/Game/AFCore/Blueprints/Game/BP_GameInstance_Main.Pegou` true _gameinstance)
  (`self.K2_DestroyActor`)
  (`/Game/AFCore/Blueprints/Game/BP_GameInstance_Main.SwitchLevel` _gameinstance "/Game/ProjetoUFPR/DataAssets/Level/DA_nivel1.DA_nivel1" true true))

(fn `UserConstructionScript`
  (`parent.UserConstructionScript`))