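; BP_BolaVida is an extra-life ball pickup that rides the BP_BallsTrack spline.
; MoveBall runs one timeline from a randomised playback position to set location along the spline, and another to add vertical offsets.
; Overlap with the left or right pincer destroys the ball and calls MostrarVidas on the game mode via AddVida.
; BolasPretas flags when no BP_BolaMorte remain, but nothing here calls it.
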(event `self.ReceiveBeginPlay`
  (bind _returnvalue (`GameplayStatics.GetActorOfClass` "/Game/ProjetoUFPR/Blueprints/BP_BallsTrack.BP_BallsTrack_C"))
  (set `self.TrackRef` _returnvalue)
  (`self.Move Ball`))

(event `Move Ball`
  (bind (_returnvalue_x _returnvalue_y _returnvalue_z) (`KismetMathLibrary.BreakVector` (`SplineComponent.GetLocationAtDistanceAlongSpline` (`/Game/ProjetoUFPR/Blueprints/BP_BallsTrack.Spline` (`self.TrackRef`)) (`KismetMathLibrary.Lerp` 0.0 (`SplineComponent.GetSplineLength` (`/Game/ProjetoUFPR/Blueprints/BP_BallsTrack.Spline` (`self.TrackRef`))) (`self.Alfa`)) "World")))
  ;[1 0 0] Evento para deixar a blinha na spline
  (`|ExecutionSequence`
    (:`then_0`
      (`TimelineComponent.SetPlaybackPosition` (`self.Ball Mover`) (`KismetMathLibrary.RandomFloatInRange` 0.0 (`SplineComponent.GetSplineLength` (`/Game/ProjetoUFPR/Blueprints/BP_BallsTrack.Spline` (`self.TrackRef`)))) false true)
      (`TimelineComponent.SetPlayRate` (`self.Ball Mover`) (/ 1.0 (`self.Duration Ball Mover`)))
      (bind (_direction _alfa) (`Timeline|Ball Mover`)
        (:`Update`
          (set `self.Alfa` _alfa)
          (`self.K2_SetActorTransform` (`KismetMathLibrary.MakeTransform` (`KismetMathLibrary.MakeVector` _returnvalue_x _returnvalue_y _returnvalue_z))))))
    (:`then_1`
      ;;[1 1 1] Playrate do Eixo Z
      (`TimelineComponent.SetPlayRate` (`self.Timeline EixoZ`) (/ 1.0 (`self.DurationEixoZ`)))
      (bind (_direction_2 _eixo_z) (`Timeline|Timeline EixoZ`)
        (:`Update`
          (bind _output_get (set `self.Eixo Z` _eixo_z))
          (`self.K2_AddActorWorldOffset` (`KismetMathLibrary.MakeVector` 0.0 0.0 _output_get)))))))

(event `BolasPretas`
  (bind _outactors (`GameplayStatics.GetAllActorsOfClass` "/Game/ProjetoUFPR/Blueprints/BP_BolaMorte.BP_BolaMorte_C"))
  (bind _returnvalue (== (`KismetArrayLibrary.Array_Length` _outactors) 0))
  (if _returnvalue
    (set `self.TemPreta` _returnvalue)))

(event `self.Colisao.OnComponentBeginOverlap`
  (params (OverlappedComponent :type "PrimitiveComponent Object Reference") (OtherActor :type "Actor Object Reference") (OtherComp :type "PrimitiveComponent Object Reference") (OtherBodyIndex :type Integer) (bFromSweep :type Boolean) (SweepResult :type "HitResult Structure (by ref)"))
  (if (or (== OtherActor (`self.Ref_PincaE`)) (== OtherActor (`self.Ref_PincaD`)))
    (cast `/Game/AFCore/Blueprints/Pawn/BP_Pawn_Base` (`GameplayStatics.GetPlayerCharacter` 0))
    (`self.K2_DestroyActor`)
    (`self.AddVida`)))

(event `AddVida`
  (bind _asbp_game_mode_main (`/Game/AFCore/Libraries/FLib_Core.getMainGameMode` (`GameplayStatics.GetGameMode`)))
  (`/Game/AFCore/Blueprints/Game/BP_GameMode_Main.Mostrar vidas` _asbp_game_mode_main))

(fn `UserConstructionScript`)