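; Tutorial ball spawner that drops blue, green and red balls near itself, then advances the game to level 1.
; After BeginPlay delays, a timed loop uses a random MultiGate to pick each ball until the counter passes its limit.
; It then polls until no "bola"-tagged actors remain, shows the pass text, resets the game mode timer and switches level.
; T destroys all balls; an uncalled-here function teleports the player to the "comecar" TargetPoint.
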(event `self.ReceiveBeginPlay`
  (bind _contador (`self.Contador`))
  (bind _returnvalue (`KismetMathLibrary.RandomPointInBoundingBox` (`self.K2_GetActorLocation` self) (5.0 5.0 0.0)))
  (`KismetSystemLibrary.Delay` 5.0)
  (bind _asbp_game_mode_main (`/Game/AFCore/Libraries/FLib_Core.getMainGameMode` (`GameplayStatics.GetGameMode`)))
  (set `/Game/AFCore/Blueprints/Game/BP_GameMode_Main.Timer` 900.0 _asbp_game_mode_main)
  (`KismetSystemLibrary.PrintString` (`KismetStringLibrary.Conv_DoubleToString` (`/Game/AFCore/Blueprints/Game/BP_GameMode_Main.Timer` _asbp_game_mode_main)))
  (`self.VisibilidadeTextos`)
  (`KismetSystemLibrary.Delay` 10.0)
  (if (> _contador 15) :!label _label
    (bind _outactors (`GameplayStatics.GetAllActorsWithTag` "bola" :!label _label_2))
    (`KismetSystemLibrary.Delay` 1.0)
    (if (== (`KismetArrayLibrary.Array_Length` _outactors) 0)
      (`SceneComponent.SetVisibility` (`self.verd`) false true)
      (`SceneComponent.SetVisibility` (`self.verm`) false true)
      (`SceneComponent.SetVisibility` (`self.azu`) false true)
      (`SceneComponent.SetVisibility` (`self.passou`) true false)
      (`KismetSystemLibrary.Delay` 5.0)
      (`SceneComponent.SetVisibility` (`self.verd`) false true)
      (`SceneComponent.SetVisibility` (`self.verm`) false true)
      (`SceneComponent.SetVisibility` (`self.azu`) false true)
      (bind _asbp_game_mode_main_2 (`/Game/AFCore/Libraries/FLib_Core.getMainGameMode` (`GameplayStatics.GetGameMode`)))
      (set `/Game/AFCore/Blueprints/Game/BP_GameMode_Main.Timer` 300.0 _asbp_game_mode_main_2)
      (bind _gameinstance (`/Game/AFCore/Libraries/FLib_Core.getMainGameInstance` (`GameplayStatics.GetGameInstance`)))
      (`/Game/AFCore/Blueprints/Game/BP_GameInstance_Main.SwitchLevel` _gameinstance "/Game/ProjetoUFPR/DataAssets/Level/DA_nivel1.DA_nivel1" false false)
      (else
        (goto _label_2)))
    (else
      (`|ExecutionSequence`
        (:`then_0`
          (goto _label_3 :!via `Reset`))
        (:`then_1`
          (`KismetSystemLibrary.PrintString` (`KismetStringLibrary.Conv_IntToString` _contador))
          (`KismetSystemLibrary.Delay` 3.0)
          (`/Engine/EditorBlueprintResources/StandardMacros.IncrementInt` (`self.Contador`)
            (:`  `
              (`|MultiGate` true :!label _label_3
                (:`Out 0`
                  (`|SpawnActorFromClass` "/Game/ProjetoUFPR/Blueprints/BP_BolaAzulTutorial.BP_BolaAzulTutorial_C" (`KismetMathLibrary.MakeTransform` _returnvalue) "AlwaysSpawn" "OverrideRootScale" null 100.0 0.0 3.0 null)
                  (goto _label))
                (:`Out 1`
                  (`|SpawnActorFromClass` "/Game/ProjetoUFPR/Blueprints/BP_BolaVerdeTutorial.BP_BolaVerdeTutorial_C" (`KismetMathLibrary.MakeTransform` _returnvalue) "AlwaysSpawn" "OverrideRootScale" null 0.0 0.0 1.0 null)
                  (goto _label))
                (:`Out 2`
                  (`|SpawnActorFromClass` "/Game/ProjetoUFPR/Blueprints/BP_BolaVermelhaTutorial.BP_BolaVermelhaTutorial_C" (`KismetMathLibrary.MakeTransform` _returnvalue) "AlwaysSpawn" "OverrideRootScale" null null)
                  (goto _label))))))))))

(event `VisibilidadeTextos`
  ;[1 1 1] Visibilidade dos textos
  (`SceneComponent.SetVisibility` (`self.passou`) false false)
  (`SceneComponent.SetVisibility` (`self.verd`) true true)
  (`SceneComponent.SetVisibility` (`self.verm`) true true)
  (`SceneComponent.SetVisibility` (`self.azu`) true true))

(event `Key|T`
  (params (Key :type "Key Structure"))
  (:`Pressed`
    (bind _outactors (`GameplayStatics.GetAllActorsWithTag` "bola"))
    (for _array_element _outactors
      (`self.K2_DestroyActor` _array_element))))

(fn `TPPaciente`
  (bind _asbp_pawn_base (cast `/Game/AFCore/Blueprints/Pawn/BP_Pawn_Base` (`GameplayStatics.GetPlayerPawn` 0)))
  (bind _outactors (`GameplayStatics.GetAllActorsOfClassWithTag` "/Script/Engine.TargetPoint" "comecar"))
  (bind _output (`|GetArrayItem` _outactors))
  (`/Game/AFCore/Blueprints/Pawn/BP_Pawn_Base.TeleportCharacter` _asbp_pawn_base (`self.K2_GetActorLocation` _output) (`self.K2_GetActorRotation` _output) null 1.0 "NewEnumerator1" true "NewEnumerator0" "NewEnumerator0" null false))

(fn `UserConstructionScript`)