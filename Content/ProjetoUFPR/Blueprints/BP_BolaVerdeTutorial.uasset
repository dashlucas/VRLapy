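; BP_BolaVerdeTutorial is a green tutorial ball meant to be picked with the correct pincer.
; Its collision overlap destroys it for the first BP_Pinca_E found, while the first BP_Pinca_D only prints a wrong-pick message.
; BeginPlay stores the starting X and Y for a timeline that would wobble the ball around that point, but nothing starts that timeline.
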(event `self.ReceiveBeginPlay`
  (bind (_returnvalue_x _returnvalue_y) (`KismetMathLibrary.BreakVector` (`SceneComponent.K2_GetComponentLocation` (`self.DefaultSceneRoot`))))
  (set `self.Return Value Y` _returnvalue_y)
  (set `self.Return Value X` _returnvalue_x))

(event `self.Colisao.OnComponentBeginOverlap`
  (params (OverlappedComponent :type "PrimitiveComponent Object Reference") (OtherActor :type "Actor Object Reference") (OtherComp :type "PrimitiveComponent Object Reference") (OtherBodyIndex :type Integer) (bFromSweep :type Boolean) (SweepResult :type "HitResult Structure (by ref)"))
  (bind _outactors (`GameplayStatics.GetAllActorsOfClass` "/Game/ProjetoUFPR/Blueprints/BP_Pinca_E.BP_Pinca_E_C"))
  (if (== OtherActor (`|GetArrayItem` _outactors))
    (`self.K2_DestroyActor`)
    (else
      (bind _outactors_2 (`GameplayStatics.GetAllActorsOfClass` "/Game/ProjetoUFPR/Blueprints/BP_Pinca_D.BP_Pinca_D_C"))
      (if (== OtherActor (`|GetArrayItem` _outactors_2))
        (`KismetSystemLibrary.PrintString` "pegou a errada")))))

(fn `UserConstructionScript`)