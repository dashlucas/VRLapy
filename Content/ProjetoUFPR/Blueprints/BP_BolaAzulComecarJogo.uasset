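; Blue start-game ball that sends the player to the starting point when both pincer actors touch it within a short window.
; Overlaps with BP_Pinca_E and BP_Pinca_D set crossed D and E flags, which clear after unequal delays.
; When both flags are true, it teleports the BP_Pawn_Base player to the TargetPoint tagged "comecar", then destroys itself after a delay.
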(event `self.ReceiveBeginPlay`
  (set `self.PincaD` false)
  (set `self.PincaE` false))

(event `self.Sphere.OnComponentBeginOverlap`
  (params (OverlappedComponent :type "PrimitiveComponent Object Reference") (OtherActor :type "Actor Object Reference") (OtherComp :type "PrimitiveComponent Object Reference") (OtherBodyIndex :type Integer) (bFromSweep :type Boolean) (SweepResult :type "HitResult Structure (by ref)"))
  (bind _outactors (`GameplayStatics.GetAllActorsOfClass` "/Game/ProjetoUFPR/Blueprints/BP_Pinca_E.BP_Pinca_E_C"))
  (if (== (`|GetArrayItem` _outactors) OtherActor)
    (`self.D_true`)
    (`self.Both_True`)
    (else
      (bind _outactors_2 (`GameplayStatics.GetAllActorsOfClass` "/Game/ProjetoUFPR/Blueprints/BP_Pinca_D.BP_Pinca_D_C"))
      (if (== OtherActor (`|GetArrayItem` _outactors_2))
        (`self.E_true`)
        (`self.Both_True`)))))

(event `D_true`
  (set `self.PincaD` true)
  (`KismetSystemLibrary.Delay` 5.0)
  (set `self.PincaD` false))

(event `E_true`
  (set `self.PincaE` true)
  (`KismetSystemLibrary.Delay` 0.5)
  (set `self.PincaE` false))

(event `Both_True`
  (if (== (`self.PincaE`) (`self.PincaD`))
    (if (== true (`self.PincaD`))
      (`self.LocalDeInicio`)
      (`KismetSystemLibrary.Delay` 1.0)
      (`self.K2_DestroyActor`))))

(fn `LocalDeInicio`
  (bind _asbp_pawn_base (cast `/Game/AFCore/Blueprints/Pawn/BP_Pawn_Base` (`GameplayStatics.GetPlayerPawn` 0)))
  (bind _outactors (`GameplayStatics.GetAllActorsOfClassWithTag` "/Script/Engine.TargetPoint" "comecar"))
  (bind _output (`|GetArrayItem` _outactors))
  (`/Game/AFCore/Blueprints/Pawn/BP_Pawn_Base.TeleportCharacter` _asbp_pawn_base (`self.K2_GetActorLocation` _output) (`self.K2_GetActorRotation` _output) null 1.0 "NewEnumerator1" true "NewEnumerator0" "NewEnumerator0" null false))

(fn `UserConstructionScript`)