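; BP_BolaVermelha1 is a red ball that scores when touched by the right pincer (BP_Pinca_D) and counts an error when touched by the left.
; Colisao overlaps compare against pincer actors, reporting to the game mode, with the correct touch destroying the ball.
; Before destruction it sets TemVerms if no BP_BolaVermelha actors exist.
; A second Sphere overlap also reports left-pincer errors; both error paths use DoOnce with a short reset delay.
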(event `self.ReceiveBeginPlay`)

(event `AddPontosRed`
  (bind _asbp_game_mode_main (`/Game/AFCore/Libraries/FLib_Core.getMainGameMode` (`GameplayStatics.GetGameMode`)))
  (`/Game/AFCore/Blueprints/Game/BP_GameMode_Main.Pontoslevel` _asbp_game_mode_main))

(event `ErrosPontosRed`
  (bind _asbp_game_mode_main (`/Game/AFCore/Libraries/FLib_Core.getMainGameMode` (`GameplayStatics.GetGameMode`)))
  (`/Game/AFCore/Blueprints/Game/BP_GameMode_Main.Erroslevel` _asbp_game_mode_main))

(event `self.Colisao.OnComponentBeginOverlap`
  (params (OverlappedComponent :type "PrimitiveComponent Object Reference") (OtherActor :type "Actor Object Reference") (OtherComp :type "PrimitiveComponent Object Reference") (OtherBodyIndex :type Integer) (bFromSweep :type Boolean) (SweepResult :type "HitResult Structure (by ref)"))
  (bind _outactors (`GameplayStatics.GetAllActorsOfClass` "/Game/ProjetoUFPR/Blueprints/BP_Pinca_D.BP_Pinca_D_C"))
  (if (== OtherActor (`|GetArrayItem` _outactors))
    (`self.BolasVerms`)
    (`self.AddPontosRed`)
    (`self.K2_DestroyActor`)
    (else
      (bind _outactors_2 (`GameplayStatics.GetAllActorsOfClass` "/Game/ProjetoUFPR/Blueprints/BP_Pinca_E.BP_Pinca_E_C"))
      (if (== OtherActor (`|GetArrayItem` _outactors_2))
        (`/Engine/EditorBlueprintResources/StandardMacros.DoOnce` false :!label _label
          (:`Completed`
            (`self.ErrosPontosRed`)
            (`KismetSystemLibrary.Delay` 0.75)
            (goto _label :!via `Reset`)))))))

(event `BolasVerms`
  (bind _outactors (`GameplayStatics.GetAllActorsOfClass` "/Game/ProjetoUFPR/Blueprints/BP_BolaVermelha.BP_BolaVermelha_C"))
  (bind _returnvalue (== (`KismetArrayLibrary.Array_Length` _outactors) 0))
  (if _returnvalue
    (set `self.TemVerms` _returnvalue)))

(event `self.Sphere.OnComponentBeginOverlap`
  (params (OverlappedComponent :type "PrimitiveComponent Object Reference") (OtherActor :type "Actor Object Reference") (OtherComp :type "PrimitiveComponent Object Reference") (OtherBodyIndex :type Integer) (bFromSweep :type Boolean) (SweepResult :type "HitResult Structure (by ref)"))
  (if (== OtherActor (`self.Ref_PincaE`))
    (`/Engine/EditorBlueprintResources/StandardMacros.DoOnce` false :!label _label_2
      (:`Completed`
        (`self.ErrosPontosRed`)
        (`KismetSystemLibrary.Delay` 0.75)
        (goto _label_2 :!via `Reset`)))))

(fn `Overlapping`
  (returns (NewParam :type Boolean))
  (return (> (`KismetArrayLibrary.Array_Length` (`PrimitiveComponent.GetOverlappingActors` (`self.Colisao`) "/Game/ProjetoUFPR/Blueprints/BP_Pinca_E.BP_Pinca_E_C")) 0)))

(fn `UserConstructionScript`)